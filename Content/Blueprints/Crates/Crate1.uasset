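; Crate1 is a breakable crate actor that bursts into flying debris when destroyed.
; AnyDamage subtracts damage from Health and destroys the actor if the result is zero or above, so the comparison appears inverted.
; The Destroyed event spawns multiple BrokenCrate actors at the crate's location in a loop, launching each one's Pieces physics bodies at high speed in a random direction.
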(event Game|Damage|EventAnyDamage
  (params (Damage :type Float%20%28single-precision%29) (DamageType :type Damage%20Type%20Object%20Reference) (InstigatedBy :type Controller%20Object%20Reference) (DamageCauser :type Actor%20Object%20Reference))
  ;[1 1 1] Destroy
  (bind _output_get (Variables|Default|Sethealth (- (Variables|Default|Gethealth) Damage)))
  (if (<= 0.0 _output_get)
    (Actor|DestroyActor)))

(event EventDestroyed
  ;[1 1 1] Destroy
  (for _index (range 0 20)
    (bind _returnvalue (Game|SpawnActorfromClass "/Game/Blueprints/Crates/BrokenCrate.BrokenCrate_C" (Math|Transform|MakeTransform (Transformation|GetActorLocation) "0, 0, 0" "1,1,1") "Undefined" 0 0))
    (Class|PrimitiveComponent|SetAllPhysicsLinearVelocity (Variables|/Game/Blueprints/Crates/BrokenCrate.BrokenCrate_C|GetPieces _returnvalue) (* (Math|Random|RandomUnitVector) 2e+03) false)))

(fn ConstructionScript)